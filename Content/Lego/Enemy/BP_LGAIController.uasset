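; BP_LGAIController is an enemy AI controller that turns perception stimuli into blackboard values.
; Stimuli tagged Noise write their location to NoisePos.
; Other stimuli are treated as sight: when successfully sensed, a living LGCharacterBase becomes Target only if the checked blackboard object is empty.
; Losing sight does not clear Target; that code is disconnected, with a note crediting a behavior tree service for the cleanup.
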(event `self.PerceptionComponent.OnPerceptionUpdated`
  (params (UpdatedActors :type "Array of Actor Object Reference (by ref)")))

(event `self.PerceptionComponent.OnTargetPerceptionUpdated`
  (params (Actor :type "Actor Object Reference") (Stimulus :type "AIStimulus Structure"))
  (bind (_age _expirationage _strength _stimuluslocation _receiverlocation _tag _bsuccessfullysensed) (break `AIStimulus` Stimulus))
  (bind _returnvalue (`AIBlueprintHelperLibrary.GetBlackboard` null))
  (if (== _tag "Noise")
    (`BlackboardComponent.SetValueAsVector` (`AIBlueprintHelperLibrary.GetBlackboard` null) (`self.NoisePos`) _stimuluslocation)
    (else
      ;[1 1 1] 视觉
      (if _bsuccessfullysensed
        (bind _aslgcharacter_base (cast `LGCharacterBase` Actor))
        (if (not (`LGCharacterBase.IsDead` _aslgcharacter_base))
          (`/Engine/EditorBlueprintResources/StandardMacros.IsValid` (`BlackboardComponent.GetValueAsObject` _returnvalue (`self.Key Name`))
            (:`Is Not Valid`
              (`BlackboardComponent.SetValueAsObject` _returnvalue (`self.Target`) Actor))))))))

(fn `UserConstructionScript`)